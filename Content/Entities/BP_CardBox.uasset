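; BP_CardBox is a card box entity with a scrapped breaking mechanic, leaving BeginPlay, Tick and the construction script empty.
; Disconnected logic caches location and speed, shows an impulse value on a text render and prints "BREAK" on sharp deceleration.
; CalSpeed and GetImpulse hold only unused math that would derive speed and its change from the box's frame-to-frame movement.
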(event EventBeginPlay
  ;[0.15 0.15 0.15 0.5] Breaking Mechnics; Scrapped.
)

(event EventTick
  (params (DeltaSeconds :type Float%20%28single-precision%29))
  ;[0.15 0.15 0.15 0.5] Breaking Mechnics; Scrapped.
)

(fn ConstructionScript)